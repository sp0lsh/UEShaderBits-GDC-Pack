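; Actor that paints density and velocity into render-target volume textures, shown on a raymarched static mesh.
; Construction creates brush material instances, seeds the targets and composites transformed shape layers into both density buffers.
; UpdatePreview, optionally ticked, feeds brush state to the materials by paint mode, ping-pongs density draws with flowmap advection settings, then triggers IBLBP's out-scatter pass.
; Smudge passes scaled velocity through the paint material; its separate smudge draw is disconnected.
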(event Custom|UpdatePreview
  (bind _paintmid (Variables|Default|GetPaintMID))
  (Rendering|Material|SetVectorParameterValue _paintmid "P" (Math|Conversions|ToLinearColor(Vector) (* (+ (/ (Variables|Internal|GetPaintLocation) 128.0) 1.0) 0.5)) :!class /Script/Engine.MaterialInstanceDynamic)
  (Rendering|Material|SetScalarParameterValue _paintmid "Trigger" (* (Variables|Default|GetTrigger%20Amount) 2.0) :!class /Script/Engine.MaterialInstanceDynamic)
  (Rendering|Material|SetScalarParameterValue _paintmid "Brush Radius" (Variables|BasicSetup|GetBrush%20Radius) :!class /Script/Engine.MaterialInstanceDynamic)
  (Rendering|Material|SetTextureParameterValue _paintmid "RT" (Utilities|Array|Get(acopy) (Variables|Internal|GetRender%20Targets) (Math|Integer|%(Integer) (+ (Variables|Default|Getidx) 1) 2)))
  (switch Utilities|FlowControl|Switch|SwitchonPaintModes (Variables|Default|GetPaint%20Mode)
    (:NewEnumerator0
      (Rendering|Material|SetVectorParameterValue (Variables|Default|GetPaintMID) "V" (Math|Color|MakeColor 0.0 0.0 0.0 0.0) :!class /Script/Engine.MaterialInstanceDynamic))
    (:NewEnumerator1
      ;[1 1 1] Velocity
      (Rendering|Material|SetVectorParameterValue (Variables|Default|GetVelocityMID) "V" (Math|Conversions|ToLinearColor(Vector) (/ (Variables|Default|GetVelocity) -256.0)) :!class /Script/Engine.MaterialInstanceDynamic)
      (Rendering|DrawMaterialtoRenderTarget "/ShaderBits-GDC-Pack/PaintingVolumeTextures/Textures/RT_Velocity.RT_Velocity" (Variables|Default|GetVelocityMID))
      (Rendering|Material|SetVectorParameterValue (Variables|Default|GetPaintMID) "V" (Math|Color|MakeColor 0.0 0.0 0.0 0.0) :!class /Script/Engine.MaterialInstanceDynamic)
      (Rendering|Material|SetScalarParameterValue (Variables|Default|GetPaintMID) "Trigger" 0.0 :!class /Script/Engine.MaterialInstanceDynamic :!label _label) ; Paint 0 strength preview
    )
    (:NewEnumerator2
      (Rendering|Material|SetVectorParameterValue (Variables|Default|GetPaintMID) "V" (Math|Conversions|ToLinearColor(Vector) (* (/ (Variables|Default|GetVelocity) -256.0) (* (Variables|Default|GetTrigger%20Amount) 2.0))) :!class /Script/Engine.MaterialInstanceDynamic)
      (goto _label)))
  (Rendering|DrawMaterialtoRenderTarget (Utilities|Array|Get(acopy) (Variables|Internal|GetRender%20Targets) (Math|Integer|%(Integer) (Variables|Default|Getidx) 2)) (Variables|Default|GetPaintMID))
  (Math|Integer|IncrementInt (Variables|Default|Getidx)
    (:%20%20
      (Utilities|IsValid (Variables|BasicSetup|GetIBL%20BP)
        (:Is%20Valid
          (Default|DrawOutScatter (Variables|BasicSetup|GetIBL%20BP)))))))

(event Custom|Clear%20and%20Seed%20RTs
  (bind _velocity_seed_material (Variables|BasicSetup|GetVelocity%20Seed%20Material))
  (Rendering|ClearRenderTarget2D (Utilities|Array|Get(acopy) (Variables|Internal|GetRender%20Targets)))
  (Rendering|ClearRenderTarget2D (Utilities|Array|Get(acopy) (Variables|Internal|GetRender%20Targets) 1))
  (Rendering|DrawMaterialtoRenderTarget (Utilities|Array|Get(acopy) (Variables|Internal|GetRender%20Targets)) (Variables|BasicSetup|GetDensity%20Seed%20Material))
  (Rendering|DrawMaterialtoRenderTarget (Utilities|Array|Get(acopy) (Variables|Internal|GetRender%20Targets) 1) (Variables|BasicSetup|GetDensity%20Seed%20Material))
  (Rendering|ClearRenderTarget2D "/ShaderBits-GDC-Pack/PaintingVolumeTextures/Textures/RT_Velocity.RT_Velocity")
  (Utilities|IsValid _velocity_seed_material
    (:Is%20Valid
      (Rendering|DrawMaterialtoRenderTarget "/ShaderBits-GDC-Pack/PaintingVolumeTextures/Textures/RT_Velocity.RT_Velocity" _velocity_seed_material))))

(event Custom|Draw%20Manual%20Layers
  (bind _render_targets (Variables|Internal|GetRender%20Targets))
  (for _array_element (Variables|ProceduralShapes|GetSliceMIDs)
    (Rendering|DrawMaterialtoRenderTarget (Utilities|Array|Get(acopy) _render_targets) _array_element)
    (Rendering|DrawMaterialtoRenderTarget (Utilities|Array|Get(acopy) _render_targets 1) _array_element)))

(event Custom|Clear%20Density
  (Rendering|ClearRenderTarget2D (Utilities|Array|Get(acopy) (Variables|Internal|GetRender%20Targets)))
  (Rendering|ClearRenderTarget2D (Utilities|Array|Get(acopy) (Variables|Internal|GetRender%20Targets) 1)))

(event Custom|Clear%20Velocity
  (Rendering|ClearRenderTarget2D "/ShaderBits-GDC-Pack/PaintingVolumeTextures/Textures/RT_Velocity.RT_Velocity"))

(event EventTick
  (params (DeltaSeconds :type Float%20%28single-precision%29))
  (if (Variables|BasicSetup|GetTick)
    (CallFunction|UpdatePreview)))

(event EventBeginPlay
  (CallFunction|ClearandSeedRTs)
  (CallFunction|DrawManualLayers))

(fn ConstructionScript
  (bind _ibl_bp (Variables|BasicSetup|GetIBL%20BP))
  (bind _returnvalue (Rendering|Material|CreateDynamicMaterialInstance (Variables|InternalMaterials|GetPaint%20Material) :!class /Script/Engine.KismetMaterialLibrary))
  (Variables|Default|SetPaintMID _returnvalue)
  (bind _returnvalue_2 (Rendering|Material|CreateDynamicMaterialInstance (Variables|InternalMaterials|GetVelocity%20Material) :!class /Script/Engine.KismetMaterialLibrary))
  (Variables|Default|SetVelocityMID _returnvalue_2)
  (bind _returnvalue_3 (Rendering|Material|CreateDynamicMaterialInstance (Variables|Default|GetSmudge%20Material) :!class /Script/Engine.KismetMaterialLibrary))
  (Variables|Default|SetSmudgeMID _returnvalue_3)
  (CallFunction|ClearandSeedRTs)
  (Rendering|Material|SetMaterial (Variables|Default|GetStaticMesh) 0 (Variables|BasicSetup|GetRaymarch%20Material))
  (CallFunction|CreateManualCompositingMIDs)
  (CallFunction|SetPaintMIDParameters)
  (CallFunction|DrawManualLayers)
  (CallFunction|UpdatePreview)
  (Default|DrawOutScatter _ibl_bp)
  (Default|DrawInternalSources _ibl_bp))

(fn CreateManualCompositingMIDs
  (bind _shape_types (Variables|ProceduralShapes|GetShape%20Types))
  (Utilities|Array|Clear (Variables|ProceduralShapes|GetSliceMIDs))
  (for (_array_element _array_index) (Variables|ProceduralShapes|GetShape%20Transforms)
    (bind _returnvalue (Rendering|Material|CreateDynamicMaterialInstance (.Material (Utilities|Struct|Break2D_Slice_Composite (Utilities|Array|Get(acopy) _shape_types (Math|Integer|Min(Integer) _array_index (Utilities|Array|LastIndex _shape_types))))) :!class /Script/Engine.KismetMaterialLibrary))
    (Rendering|Material|SetTextureParameterValue _returnvalue "Texture" (.Texture (Utilities|Struct|Break2D_Slice_Composite (Utilities|Array|Get(acopy) _shape_types (Math|Integer|Min(Integer) _array_index (Utilities|Array|LastIndex _shape_types))))))
    (Rendering|Material|SetScalarParameterValue _returnvalue "R" (/ (.Yaw (Math|Rotator|BreakRotator (.Rotation (Math|Transform|BreakTransform _array_element)))) -3.6e+02) :!class /Script/Engine.MaterialInstanceDynamic)
    (Rendering|Material|SetVectorParameterValue _returnvalue "P" (Math|Conversions|ToLinearColor(Vector) (* (+ (/ (.Location (Math|Transform|BreakTransform _array_element)) 128.0) 1.0) 0.5)) :!class /Script/Engine.MaterialInstanceDynamic)
    (Rendering|Material|SetVectorParameterValue _returnvalue "S" (Math|Conversions|ToLinearColor(Vector) (Math|Vector|MakeVector (.X (Math|Vector|BreakVector (.Scale (Math|Transform|BreakTransform _array_element)))) (.Y (Math|Vector|BreakVector (.Scale (Math|Transform|BreakTransform _array_element)))) (Math|Float|Max(Float) (.Z (Math|Vector|BreakVector (.Scale (Math|Transform|BreakTransform _array_element)))) 0.0))) :!class /Script/Engine.MaterialInstanceDynamic)
    (Utilities|Array|Add (Variables|ProceduralShapes|GetSliceMIDs) _returnvalue)))

(fn SetPaintMIDParameters
  (Rendering|Material|SetScalarParameterValue (Variables|Default|GetPaintMID) "Advection Speed" (Variables|FlowmapSettings|GetFlowmap%20Speed) :!class /Script/Engine.MaterialInstanceDynamic)
  (Rendering|Material|SetScalarParameterValue (Variables|Default|GetPaintMID) "Flowmap Strength" (Variables|FlowmapSettings|GetFlowmap%20Strength) :!class /Script/Engine.MaterialInstanceDynamic)
  (Rendering|Material|SetScalarParameterValue (Variables|Default|GetPaintMID) "Steps" (Math|Conversions|ToFloat(Integer) (Variables|FlowmapSettings|GetFlowmap%20Iterations)) :!class /Script/Engine.MaterialInstanceDynamic))

(fn GrabPressed*
  (params (Which%20Hand :type LeftRight%20Enum :default "NewEnumerator0") (Hand%20BP :type BP%20Left%20Hand%20Object%20Reference))
  (return "" false false "0, 0, 0"))

(fn GrabReleased*
  (params (Which%20Hand :type LeftRight%20Enum :default "NewEnumerator0"))
  (return false))

(fn HandBeginOverlap*
  (params (Which%20Hand :type LeftRight%20Enum :default "NewEnumerator0") (Hand%20BP :type BP%20Left%20Hand%20Object%20Reference))
  (return false 0))

(fn HandEndOverlap*
  (params (Which%20Hand :type LeftRight%20Enum :default "NewEnumerator0"))
  (return false))

(fn TriggerPressed*
  (params (Which%20Hand :type LeftRight%20Enum :default "NewEnumerator0") (Hand%20BP :type BP%20Left%20Hand%20Object%20Reference))
  (return false))

(fn TriggerReleased*
  (params (Which%20Hand :type LeftRight%20Enum :default "NewEnumerator0"))
  (return false))
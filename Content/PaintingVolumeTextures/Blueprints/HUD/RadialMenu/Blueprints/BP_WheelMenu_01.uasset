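; Motion-controller radial wheel menu, for either hand, that navigates nested categories and sends mode or action changes to the player pawn.
; Widget class defaults define each level, spawned in a circle as text plus sprite, mesh or child-actor icons, with automatic Back buttons.
; Tick converts stick axes from a Material Parameter Collection into the hovered slot.
; A parent stack handles going back; override events temporarily swap the menu root.
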(event Custom|Menu%20Override
  (params (Widget :type Radial%20Menu%20BP%20Widget%20Class%20Class%20Reference))
  (bind _parentstack (Variables|Default|GetParentStack))
  ;[1 1 1] External Mode Force
  (Variables|Default|SetOldParentStack _parentstack)
  (Utilities|Array|Clear _parentstack)
  (Variables|Default|SetOldRoot (Variables|Default|GetRootWidget))
  (Variables|Default|SetOldWidget (Variables|Default|GetCurrentWidget))
  (bind _output_get (Variables|Default|SetCurrentWidget Widget))
  (Variables|Default|SetRootWidget _output_get)
  ;[1 1 1] Select
  (Utilities|SelectWidget (Variables|Default|GetCurrentWidgets) (.WidgetType (Utilities|Struct|BreakRadialMenu_Widget_Component_Struct (Utilities|Array|Get(acopy) (Variables|Default|GetCurrentWidgets) (Variables|Default|GetCurrentSelection))))
    (:Out
      (Variables|Default|SetCurrentSelection -1))))

(event Custom|Menu%20Select
  (bind _parentstack (Variables|Default|GetParentStack))
  (bind _returnvalue (Utilities|Array|LastIndex _parentstack))
  ;[1 0 0.006724] Selection Logic
  (Utilities|UpdateChildActorVisibility false
    (:Out
      (if (>= (Variables|Default|GetCurrentSelection) 0) ; Any selection
        ;[1 1 1] Canel
        (switch Utilities|FlowControl|Switch|SwitchonE_RadialMenu_Widget_Types (.WidgetType (Utilities|Struct|BreakRadialMenu_WidgetInfo_Struct (.WidgetInfo (Utilities|Struct|BreakRadialMenu_Widget_Component_Struct (Utilities|Array|Get(acopy) (Variables|Default|GetCurrentWidgets) (Variables|Default|GetCurrentSelection))))))
          (:NewEnumerator0
            ;[1 1 1] Select
            (Utilities|Array|Add (Variables|Default|GetParentStack) (Variables|Default|GetCurrentWidget))
            (Variables|Default|SetCurrentWidget (.WidgetType (Utilities|Struct|BreakRadialMenu_Widget_Component_Struct (Utilities|Array|Get(acopy) (Variables|Default|GetCurrentWidgets) (Variables|Default|GetCurrentSelection)))))
            (Utilities|SelectWidget (Variables|Default|GetCurrentWidgets) (.WidgetType (Utilities|Struct|BreakRadialMenu_Widget_Component_Struct (Utilities|Array|Get(acopy) (Variables|Default|GetCurrentWidgets) (Variables|Default|GetCurrentSelection)))) :!label _label
              (:Out
                (Variables|Default|SetCurrentSelection -1))))
          (:NewEnumerator1
            (goto _label))
          (:NewEnumerator2
            (if (== (.WidgetType (Utilities|Struct|BreakRadialMenu_Widget_Component_Struct (Utilities|Array|Get(acopy) (Variables|Default|GetCurrentWidgets) (Variables|Default|GetCurrentSelection)))) "/ShaderBits-GDC-Pack/PaintingVolumeTextures/Blueprints/HUD/RadialMenu/Blueprints/Buttons/UI_Button_Back.UI_Button_Back_C") ; Go back if Back
              (Development|PrintString "BACK")
              ;[1 1 1] Go Up a level
              (bind _output_get (Variables|Default|SetCurrentWidget (Utilities|Array|Get(acopy) _parentstack _returnvalue)))
              (Utilities|SelectWidget (Variables|Default|GetCurrentWidgets) _output_get
                (:Out
                  (Utilities|Array|RemoveIndex (Variables|Default|GetParentStack) _returnvalue)
                  (Variables|Default|SetCurrentSelection -1)))))
          (:NewEnumerator3
            (goto _label)))))))

(event Custom|Manual%20Selection
  (params (idx :type Integer))
  (bind _parentstack (Variables|Default|GetParentStack))
  (bind _returnvalue (Utilities|Array|LastIndex _parentstack))
  (Variables|Default|SetCurrentSelection idx)
  ;[1 0 0.006724] Selection Logic
  (Utilities|UpdateChildActorVisibility false
    (:Out
      (if (>= (Variables|Default|GetCurrentSelection) 0) ; Any selection
        ;[1 1 1] Canel
        (switch Utilities|FlowControl|Switch|SwitchonE_RadialMenu_Widget_Types (.WidgetType (Utilities|Struct|BreakRadialMenu_WidgetInfo_Struct (.WidgetInfo (Utilities|Struct|BreakRadialMenu_Widget_Component_Struct (Utilities|Array|Get(acopy) (Variables|Default|GetCurrentWidgets) (Variables|Default|GetCurrentSelection))))))
          (:NewEnumerator0
            ;[1 1 1] Select
            (Utilities|Array|Add (Variables|Default|GetParentStack) (Variables|Default|GetCurrentWidget))
            (Variables|Default|SetCurrentWidget (.WidgetType (Utilities|Struct|BreakRadialMenu_Widget_Component_Struct (Utilities|Array|Get(acopy) (Variables|Default|GetCurrentWidgets) (Variables|Default|GetCurrentSelection)))))
            (Utilities|SelectWidget (Variables|Default|GetCurrentWidgets) (.WidgetType (Utilities|Struct|BreakRadialMenu_Widget_Component_Struct (Utilities|Array|Get(acopy) (Variables|Default|GetCurrentWidgets) (Variables|Default|GetCurrentSelection)))) :!label _label
              (:Out
                (Variables|Default|SetCurrentSelection -1))))
          (:NewEnumerator1
            (goto _label))
          (:NewEnumerator2
            (if (== (.WidgetType (Utilities|Struct|BreakRadialMenu_Widget_Component_Struct (Utilities|Array|Get(acopy) (Variables|Default|GetCurrentWidgets) (Variables|Default|GetCurrentSelection)))) "/ShaderBits-GDC-Pack/PaintingVolumeTextures/Blueprints/HUD/RadialMenu/Blueprints/Buttons/UI_Button_Back.UI_Button_Back_C") ; Go back if Back
              (Development|PrintString "BACK")
              ;[1 1 1] Go Up a level
              (bind _output_get (Variables|Default|SetCurrentWidget (Utilities|Array|Get(acopy) _parentstack _returnvalue)))
              (Utilities|SelectWidget (Variables|Default|GetCurrentWidgets) _output_get
                (:Out
                  (Utilities|Array|RemoveIndex (Variables|Default|GetParentStack) _returnvalue)
                  (Variables|Default|SetCurrentSelection -1)))))
          (:NewEnumerator3
            (goto _label)))))))

(event Custom|End%20Menu%20Override
  ;[1 1 1] End Override and restore menu state
  (Variables|Default|SetParentStack (Variables|Default|GetOldParentStack))
  (Variables|Default|SetRootWidget (Variables|Default|GetOldRoot))
  (Variables|Default|SetCurrentWidget (Variables|Default|GetOldWidget))
  ;[1 1 1] Select
  (Utilities|SelectWidget (Variables|Default|GetCurrentWidgets) (.WidgetType (Utilities|Struct|BreakRadialMenu_Widget_Component_Struct (Utilities|Array|Get(acopy) (Variables|Default|GetCurrentWidgets) (Variables|Default|GetCurrentSelection))))
    (:Out
      (Variables|Default|SetCurrentSelection -1))))

(event Custom|Trigger%20Release
  (params (Hand :type Byte :default 0))
  (if (Variables|Default|GetRightHand)
    _))

(event Custom|Right%20Trigger%20Release
  (if (Variables|Default|GetRightHand)
    _))

(event EventBeginPlay
  ;[1 1 1] Find Other Components
  (Utilities|FlowControl|Delay 0.5)
  (CallFunction|InitialSetup))

(event EventTick
  (params (DeltaSeconds :type Float%20%28single-precision%29))
  (if (not (Variables|Rendering|GetbHidden))
    (bind _returnvalue (Rendering|Material|GetVectorParameterValue "/ShaderBits-GDC-Pack/PaintingVolumeTextures/Blueprints/HUD/Controllers/Materials/MPC_MotionControllers.MPC_MotionControllers" (select (Variables|Default|GetRightHand) (Utilities|Name|MakeLiteralName "RightStickAxis") (Utilities|Name|MakeLiteralName "LeftStickAxis")) :!class /Script/Engine.KismetMaterialLibrary))
    ;[1 0 0.006724] Selection Logic
    (if (not (< (.Z (Math|Vector|BreakVector (Math|Conversions|ToVector(LinearColor) _returnvalue))) 0.55))
      (Utilities|UpdateChildActorVisibility true
        (:Out
          ;[1 1 1] Selection based off Axis
          (Variables|Default|SetCurrentSelection (Math|Float|Truncate (* (Math|Float|Fraction (+ (+ (/ (Math|Trig|Atan2(Radians) (select (Variables|Default|GetRightHand) (* (.X (Math|Vector|BreakVector (Math|Conversions|ToVector(LinearColor) _returnvalue))) -1.0) (* (.X (Math|Vector|BreakVector (Math|Conversions|ToVector(LinearColor) _returnvalue))) -1.0)) (select (Variables|Default|GetRightHand) (* (.Y (Math|Vector|BreakVector (Math|Conversions|ToVector(LinearColor) _returnvalue))) 1.0) (.Y (Math|Vector|BreakVector (Math|Conversions|ToVector(LinearColor) _returnvalue))))) (* (Math|Trig|GetPI) 2.0)) 0.5) (* (/ 1.0 (Math|Conversions|ToFloat(Integer) (Utilities|Array|Length (Variables|Default|GetCurrentWidgets)))) 0.5))) (Math|Conversions|ToFloat(Integer) (Utilities|Array|Length (Variables|Default|GetCurrentWidgets))))))
          ;[1 1 1] Current Hover Highlight
          (Utilities|AddWidgetHoverHighlight (Utilities|Array|Get(acopy) (Variables|Default|GetCurrentWidgets) (Variables|Default|GetCurrentSelection))
            (:Out
              ;[1 1 1] Deselect Before and After Widgets
              (Utilities|RemoveWidgetHighlight (Utilities|Array|Get(acopy) (Variables|Default|GetCurrentWidgets) (Math|Integer|SelectInt (Utilities|Array|LastIndex (Variables|Default|GetCurrentWidgets)) (Math|Integer|%(Integer) (+ (Variables|Default|GetCurrentSelection) -1) (Utilities|Array|Length (Variables|Default|GetCurrentWidgets))) (<= (Variables|Default|GetCurrentSelection) 0)))
                (:Out
                  (Utilities|RemoveWidgetHighlight (Utilities|Array|Get(acopy) (Variables|Default|GetCurrentWidgets) (Math|Integer|%(Integer) (+ (Variables|Default|GetCurrentSelection) 1) (Utilities|Array|Length (Variables|Default|GetCurrentWidgets))))))))))))))

(fn ConstructionScript
  (Rendering|Material|SetVectorParameterValue "/ShaderBits-GDC-Pack/PaintingVolumeTextures/Blueprints/HUD/Controllers/Materials/MPC_MotionControllers.MPC_MotionControllers" "LeftStickAxis" (Math|Color|MakeColor 0.0 0.0 1.0) :!class /Script/Engine.KismetMaterialLibrary) ; Make Menu Visible for Debug Only
  (CallFunction|InitialSetup))

(fn CreateWidgets
  (params (WidgetInfo :type Radial%20Menu%20Widget%20Info%20Struct%20Structure) (WidgetType :type Radial%20Menu%20BP%20Widget%20Class%20Class%20Reference) (Location :type Vector) (idx :type Integer))
  (bind _returnvalue (+ Location "0.000000,15.000000,2.000000"))
  (bind _returnvalue_2 (Math|Transform|MakeTransform _returnvalue "90.000000,0.000000,90.000000"))
  ;[1 1 1] Add Text
  (LocalVariables|SetCurWidgInfo WidgetInfo)
  (LocalVariables|SetCurWidgType WidgetType)
  (bind _returnvalue_3 (AddComponent|AddTextRenderComponent false (Math|Transform|MakeTransform (- Location "0.000000,10.000000,-1.000000") "90.000000, 0,90.000000" "0.500000,0.500000,0.500000")))
  (Class|TextRenderComponent|SetTextMaterial _returnvalue_3 (select (Variables|Default|GetRightHand) "/ShaderBits-GDC-Pack/PaintingVolumeTextures/Blueprints/HUD/RadialMenu/Materials/M_RadialMenuText_01_RightHandMenu.M_RadialMenuText_01_RightHandMenu" "/ShaderBits-GDC-Pack/PaintingVolumeTextures/Blueprints/HUD/RadialMenu/Materials/M_RadialMenuText_01.M_RadialMenuText_01"))
  (bind _output_get (LocalVariables|SetTextComponent _returnvalue_3))
  (Rendering|Components|TextRender|SetText _output_get (Utilities|Text|ToText(String) (Utilities|String|Append (.WidgetModeName (Utilities|Struct|BreakRadialMenu_WidgetInfo_Struct (LocalVariables|GetCurWidgInfo))) (Utilities|String|ToString(Integer) idx))))
  ;[1 1 1] Add Simple Sprite
  (switch Utilities|FlowControl|Switch|SwitchonE_RadialMenu_ObjectTypes (.Object_Type (Utilities|Struct|BreakRadialMenu_WidgetInfo_Struct (LocalVariables|GetCurWidgInfo)))
    (:NewEnumerator5
      (bind _returnvalue_4 (AddComponent|AddStaticMeshComponent false (Math|Transform|MakeTransform _returnvalue "0,180.000000,0.000000" "25.000000,25.000000,25.000000") :!label _label))
      (bind _output_get_2 (LocalVariables|SetMeshComponent _returnvalue_4))
      (bind _returnvalue_5 (Rendering|Material|CreateDynamicMaterialInstance _output_get_2 0 (select (Variables|Default|GetRightHand) "/ShaderBits-GDC-Pack/PaintingVolumeTextures/Blueprints/HUD/RadialMenu/Materials/WidgetMaterial_RightHandMenu.WidgetMaterial_RightHandMenu" "/ShaderBits-GDC-Pack/PaintingVolumeTextures/Blueprints/HUD/RadialMenu/Materials/WidgetMaterial.WidgetMaterial") :!class /Script/Engine.PrimitiveComponent))
      (Rendering|Material|SetTextureParameterValue _returnvalue_5 "Texture" (Utilities|ResolveSoftReference (.SpriteTex (Utilities|Struct|BreakRadialMenu_WidgetInfo_Struct (LocalVariables|GetCurWidgInfo)))))
      ;[1 1 1] Encode Widget Component
      (Utilities|Array|Add (Variables|Default|GetCurrentWidgets) (Utilities|Struct|MakeRadialMenu_Widget_Component_Struct (LocalVariables|GetMeshComponent) (LocalVariables|GetTextComponent) (LocalVariables|GetCurWidgType) _returnvalue_5 false (LocalVariables|GetCurWidgInfo) (Transformation|GetWorldScale _returnvalue_4))))
    (:NewEnumerator1
      (if (.ClassSpawnInMenu (Utilities|Struct|BreakRadialMenu_WidgetInfo_Struct (LocalVariables|GetCurWidgInfo)))
        (Utilities|FlowControl|Sequence
          (:then_0
            (bind _returnvalue_6 (AddComponent|AddStaticMeshComponent false (Math|Transform|MakeTransform _returnvalue "0.000000,180.000000,0.000000" "45.000000,45.000000,45.000000")))
            (bind _output_get_3 (LocalVariables|SetMeshComponent _returnvalue_6))
            (bind _returnvalue_7 (Rendering|Material|CreateDynamicMaterialInstance _output_get_3 0 (select (Variables|Default|GetRightHand) "/ShaderBits-GDC-Pack/PaintingVolumeTextures/Blueprints/HUD/RadialMenu/Materials/ActorClassHighlight_RightHandMenu.ActorClassHighlight_RightHandMenu" "/ShaderBits-GDC-Pack/PaintingVolumeTextures/Blueprints/HUD/RadialMenu/Materials/ActorClassHighlight.ActorClassHighlight") :!class /Script/Engine.PrimitiveComponent)))
          (:then_1
            ;[1 1 1] Class
            (bind _asactor (Utilities|Casting|CastToActorClass (.Class (Utilities|Struct|BreakRadialMenu_WidgetInfo_Struct (LocalVariables|GetCurWidgInfo))))
              (:then
                (bind _returnvalue_8 (AddComponent|AddChildActorComponent false _returnvalue_2))
                (Utilities|IsValid _returnvalue_8
                  (:Is%20Valid
                    (ChildActorComponent|SetChildActorClass _returnvalue_8 _asactor)
                    (Transformation|SetRelativeScale3D _returnvalue_8 "0.100000,0.100000,0.100000"))
                  (:Is%20Not%20Valid
                    _))
                (Development|PrintString "Hello"))
              (:CastFailed
                _))
            ;[1 1 1] Encode Widget Component
            (Utilities|Array|Add (Variables|Default|GetCurrentWidgets) (Utilities|Struct|MakeRadialMenu_Widget_Component_Struct (LocalVariables|GetMeshComponent) (LocalVariables|GetTextComponent) (LocalVariables|GetCurWidgType) _returnvalue_7 false (LocalVariables|GetCurWidgInfo) (Transformation|GetWorldScale _returnvalue_6) _returnvalue_8 (Transformation|GetWorldScale _returnvalue_8)))
            (Utilities|Array|Add (Variables|Default|GetChildActorsForVisControl) _returnvalue_8)))
        (else
          (goto _label))))
    (:NewEnumerator0
      ;[1 1 1] Add Static Mesh
      (bind _returnvalue_9 (AddComponent|AddStaticMeshComponent false _returnvalue_2))
      (bind _output_get_4 (LocalVariables|SetMeshComponent _returnvalue_9))
      (Components|StaticMesh|SetStaticMesh _output_get_4 (.StaticMesh (Utilities|Struct|BreakRadialMenu_WidgetInfo_Struct (LocalVariables|GetCurWidgInfo))))
      (Transformation|SetRelativeScale3D (LocalVariables|GetMeshComponent) (* (Math|Conversions|ToVector(Float) (* (/ 1.0 (.SphereRadius (Collision|GetComponentBounds _returnvalue_9))) 25.0)) (Transformation|GetWorldScale (Variables|Default|GetScene))))
      (bind _returnvalue_10 (Rendering|Material|CreateDynamicMaterialInstance (LocalVariables|GetMeshComponent) 0 (select (Variables|Default|GetRightHand) "/ShaderBits-GDC-Pack/PaintingVolumeTextures/Blueprints/HUD/RadialMenu/Materials/M_Meshmaterial_RightHandMenu.M_Meshmaterial_RightHandMenu" "/ShaderBits-GDC-Pack/PaintingVolumeTextures/Blueprints/HUD/RadialMenu/Materials/M_Meshmaterial.M_Meshmaterial") :!class /Script/Engine.PrimitiveComponent))
      (for _index (range 0 (Rendering|Material|GetNumMaterials (LocalVariables|GetMeshComponent)))
        (Rendering|Material|SetMaterial (LocalVariables|GetMeshComponent) _index _returnvalue_10))
      ;[1 1 1] Encode Widget Component
      (Utilities|Array|Add (Variables|Default|GetCurrentWidgets) (Utilities|Struct|MakeRadialMenu_Widget_Component_Struct (LocalVariables|GetMeshComponent) (LocalVariables|GetTextComponent) (LocalVariables|GetCurWidgType) _returnvalue_10 false (LocalVariables|GetCurWidgInfo) (Transformation|GetWorldScale (LocalVariables|GetMeshComponent)))))))

(fn InitialSetup
  (bind _output_get (Variables|Default|SetCurrentWidget (Variables|Default|GetRootWidget)))
  (bind _new_widgets (Utilities|ClearandDisplayWidgets (Variables|Default|GetCurrentWidgets) (.Sub%20Widgets (Utilities|GetClassDefaults _output_get)))
    (:Done
      (Variables|Default|SetCurrentWidgets _new_widgets)
      (Variables|Default|SetPawn (Game|Player|GetPlayerPawn 0))
      ;[1 1 1] Right Hand Material Swaps
      (if (Variables|Default|GetRightHand)
        (Rendering|Material|SetMaterial (Variables|Default|GetWheelMenuMesh) 0 "/ShaderBits-GDC-Pack/PaintingVolumeTextures/Blueprints/HUD/RadialMenu/Materials/M_WheelMenu_01_RightHandMenu.M_WheelMenu_01_RightHandMenu"))
      (return))))
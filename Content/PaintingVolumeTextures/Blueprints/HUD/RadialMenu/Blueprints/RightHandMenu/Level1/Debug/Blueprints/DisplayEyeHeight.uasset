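; Debug display actor in the right-hand radial menu that shows the user's eye height as text.
; Its construction script reads EyeHeightInches and HeadLocalZ from the MPC_UI material parameter collection.
; It writes the local Z value, plus eye height split into feet and inches, to a TextRender component.
; The text is set only at construction, with no active Tick or event logic to refresh it.
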(event EventBeginPlay)

(event Collision|EventActorBeginOverlap
  (params (OtherActor :type Actor%20Object%20Reference)))

(event EventTick
  (params (DeltaSeconds :type Float%20%28single-precision%29)))

(fn ConstructionScript
  (bind _returnvalue (Rendering|Material|GetScalarParameterValue "/ShaderBits-GDC-Pack/PaintingVolumeTextures/Blueprints/HUD/RadialMenu/Materials/MPC_UI.MPC_UI" "EyeHeightInches" :!class /Script/Engine.KismetMaterialLibrary))
  (bind _returnvalue_2 (Rendering|Material|GetScalarParameterValue "/ShaderBits-GDC-Pack/PaintingVolumeTextures/Blueprints/HUD/RadialMenu/Materials/MPC_UI.MPC_UI" "HeadLocalZ" :!class /Script/Engine.KismetMaterialLibrary))
  (Rendering|Components|TextRender|SetText (Variables|Default|GetTextRender) (Utilities|Text|ToText(String) (Utilities|String|Append (Utilities|String|Append (Utilities|String|Append (Utilities|String|ToString(Text) (Utilities|Text|ToText(Float) _returnvalue_2 "HalfToEven" true 3 3 1 1)) "local Z,   ") (Utilities|String|Append (Utilities|String|ToString(Integer) (Math|Float|Floor (/ _returnvalue 12.0))) "ft ")) (Utilities|String|Append (Utilities|String|ToString(Float) (Math|Float|%(Float) _returnvalue 12.0)) "in")))))